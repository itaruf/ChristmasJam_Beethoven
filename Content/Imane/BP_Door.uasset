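; Door that the player opens by clearing a series of random-key quick-time events while inside its trigger box.
; Entering the box starts a looping timer that reads the player's event state and has the BP_GMB game mode start each next QTE.
; Clearing the count plays a timeline that yaws the door 90 degrees.
; A wrong key, timeout or leaving mid-event fails the sequence, clearing the timer and widget.
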(event OnComponentBeginOverlap(BoxOpenDoorRange)
  (params (OverlappedComponent :type Primitive%20Component%20Object%20Reference) (OtherActor :type Actor%20Object%20Reference) (OtherComp :type Primitive%20Component%20Object%20Reference) (OtherBodyIndex :type Integer) (bFromSweep :type Boolean) (SweepResult :type Hit%20Result%20Structure%20%28by%20ref%29))
  ;[1 1 1] Actor Begin Overlap - Start QTE
  (if (Variables|Default|GetbCanOpen)
    (bind _asfirst_person_character (Utilities|Casting|CastToFirstPersonCharacter OtherActor))
    (Variables|Default|SetPlayer _asfirst_person_character)
    (Utilities|FlowControl|Sequence
      (:then_0
        ;[1 1 1] Reset State When Entering
        (Variables|Default|SetNumberOfQTELeft (Variables|Default|GetNumberOfQTE))
        (Variables|Default|SetEventWidgetPosition (Utilities|Struct|Makes_EventWidgetPosition (Utilities|Struct|MakeAnchors "(X=0.500000,Y=0.500000)" "(X=0.500000,Y=0.500000)") "(X=0.500000,Y=0.500000)" "(X=0.000000,Y=0.000000)")))
      (:then_1
        (Utilities|IsValid (Variables|Default|GetPlayer)
          (:Is%20Valid
            (Utilities|Struct|Setmembersins_EventInfo (Variables|/Game/FirstPersonCPP/Blueprints/FirstPersonCharacter.FirstPersonCharacter_C|GetCurrentEvent (Variables|Default|GetPlayer)) "NewEnumerator0"))))
      (:then_2
        ;[1 1 1] Repeat QTE Every X Seconds
        (bind _returnvalue (Utilities|Time|SetTimerbyEvent (delegate Custom|QTE) 0.5 true))
        (Variables|Default|SetLoop _returnvalue)))))

(event OnComponentEndOverlap(BoxOpenDoorRange)
  (params (OverlappedComponent :type Primitive%20Component%20Object%20Reference) (OtherActor :type Actor%20Object%20Reference) (OtherComp :type Primitive%20Component%20Object%20Reference) (OtherBodyIndex :type Integer))
  ;[1 1 1] Actor End Overlap - Stop QTE > Set State To Failure
  (if (Variables|Default|GetbCanOpen)
    (Variables|Default|SetNumberOfQTELeft (Variables|Default|GetNumberOfQTE))
    (Utilities|FlowControl|Sequence
      (:then_0
        (bind _asfirst_person_character (Utilities|Casting|CastToFirstPersonCharacter OtherActor))
        (Variables|Default|SetPlayer _asfirst_person_character)
        (bind _asbp_gmb (Utilities|Casting|CastToBP_GMB (Game|GetGameMode)))
        (Variables|Default|SetGMB _asbp_gmb)
        (Components|Activation|Activate (Variables|/Script/Engine.Character|GetCharacterMovement (Variables|Default|GetPlayer)) false)
        (Variables|/Game/Imane/BP_GMB.BP_GMB_C|SetbQTEended (Variables|Default|GetGMB) true))
      (:then_1
        (switch Utilities|FlowControl|Switch|Switchone_EventState (Utilities|Struct|Breaks_EventInfo (Variables|/Game/FirstPersonCPP/Blueprints/FirstPersonCharacter.FirstPersonCharacter_C|GetCurrentEvent (Variables|Default|GetPlayer)))
          (:NewEnumerator0
            _)
          (:NewEnumerator1
            _))
        (Default|OnEventCompleted (Variables|Default|GetPlayer) "NewEnumerator3")
        (CallFunction|Failure "NewEnumerator3")))))

(event Custom|QTE
  (bind _player (Variables|Default|GetPlayer))
  (bind _currentevent (Variables|/Game/FirstPersonCPP/Blueprints/FirstPersonCharacter.FirstPersonCharacter_C|GetCurrentEvent _player))
  (bind _state (Utilities|Struct|Breaks_EventInfo _currentevent))
  ;[1 1 1] Repeat QTE Every X Seconds
  (Utilities|IsValid _player
    (:Is%20Valid
      (switch Utilities|FlowControl|Switch|Switchone_EventState _state
        (:NewEnumerator0
          (if (Variables|/Game/Imane/BP_GMB.BP_GMB_C|GetbQTEended (Variables|Default|GetGMB)) :!label _label
            (Math|Integer|DecrementInt (Variables|Default|GetNumberOfQTELeft)
              (:%20%20
                (Variables|/Game/Imane/BP_GMB.BP_GMB_C|SetbQTEended (Variables|Default|GetGMB) false)
                (if (== (Variables|Default|GetNumberOfQTELeft) 0)
                  ;[1 1 1] If The Player Has Cleared All QTE - Open The Door
                  (Utilities|Time|ClearandInvalidateTimerbyHandle (Variables|Default|GetLoop))
                  (CallFunction|OpenDoor)
                  (Variables|Default|SetbCanOpen false)
                  (Variables|/Game/Imane/BP_GMB.BP_GMB_C|SetbQTEended (Variables|Default|GetGMB) true)
                  (Components|Activation|Activate (Variables|/Script/Engine.Character|GetCharacterMovement (Variables|Default|GetPlayer)) true)
                  (else
                    ;[1 1 1] Start QTE With Key To Press
                    (Default|StartQTE (Variables|Default|GetGMB) (Variables|Default|GetPlayer) (.OutItem (Utilities|Array|Random (Variables|Default|GetRandom%20Keys))) (Variables|Default|GetEventWidgetPosition) (Variables|Default|GetTime) 1.0)))))))
        (:NewEnumerator1
          (goto _label))
        (:NewEnumerator2
          (goto _label))
        (:NewEnumerator3
          (CallFunction|Failure _state)
          (Components|Activation|Activate (Variables|/Script/Engine.Character|GetCharacterMovement (Variables|Default|GetPlayer)) true :!label _label_2))
        (:NewEnumerator4
          (CallFunction|Failure _state)
          (goto _label_2))))))

(event Custom|OpenDoor
  ;[1 1 1] Open Door / Close Door
  (Variables|Default|SetDoorRotation (Transformation|GetWorldRotation (Variables|Default|GetDefaultSceneRoot)))
  (bind _open (Timeline|Open Play)
    (:Update
      (Transformation|SetWorldRotation (Variables|Default|GetDefaultSceneRoot) (Math|Rotator|Lerp(Rotator) (Variables|Default|GetDoorRotation) (CallFunction|CalculateNewDoorRotation) _open) false false))))

(event EventBeginPlay
  ;[1 1 1] Retrieve Data
  (Utilities|FlowControl|Sequence
    (:then_0
      (bind _asfirst_person_character (Utilities|Casting|CastToFirstPersonCharacter (Pawn|GetControlledPawn (Game|GetPlayerController 0))))
      (Variables|Default|SetPlayer _asfirst_person_character)
      (bind _asbp_gmb (Utilities|Casting|CastToBP_GMB (Game|GetGameMode)))
      (Variables|Default|SetGMB _asbp_gmb))
    (:then_1
      (Variables|Default|SetRandom%20Keys (Variables|/Game/FirstPersonCPP/Blueprints/FirstPersonCharacter.FirstPersonCharacter_C|GetRandomKeys (Variables|Default|GetPlayer))))))

(event EventTick
  (params (DeltaSeconds :type Float%20%28single-precision%29))
  ;[1 1 1] Open Door / Close Door
  (Variables|Default|SetbCanOpen (< (stale Custom|OpenDoor _open) 1.0)))

(fn ConstructionScript)

(fn CalculateNewDoorRotation
  (bind _doorrotation (Variables|Default|GetDoorRotation))
  (bind (_roll _pitch _yaw) (Math|Rotator|BreakRotator _doorrotation))
  (return (Math|Rotator|MakeRotator _roll _pitch (+ _yaw -9e+01))))

(fn Failure
  (params (State :type e_EventState%20Enum :default "NewEnumerator0"))
  (bind _player (Variables|Default|GetPlayer))
  (bind _eventwidget (Variables|/Game/FirstPersonCPP/Blueprints/FirstPersonCharacter.FirstPersonCharacter_C|GetEventWidget _player))
  (Default|OnEventCompleted (Variables|Default|GetPlayer) State)
  (Utilities|FlowControl|Sequence
    (:then_0
      (Variables|/Game/Imane/BP_GMB.BP_GMB_C|SetbQTEended (Variables|Default|GetGMB) true)
      (if (Utilities|Time|IsValidTimerHandle (Variables|Default|GetLoop))
        (Utilities|Time|ClearandInvalidateTimerbyHandle (Variables|Default|GetLoop))))
    (:then_1
      (Utilities|IsValid _eventwidget
        (:Is%20Valid
          (Widget|RemovefromParent _eventwidget))))))