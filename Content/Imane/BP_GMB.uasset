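; BP_GMB runs the game's countdown and flags game over when time runs out.
; On BeginPlay it hides the mouse cursor and starts a looping one-second timer that decrements Seconds.
; When Seconds is zero, it decrements Minutes but sets Seconds to 0 rather than 59, so remaining minutes drop one per tick.
; With both at zero it sets GameOver, and the timer keeps running.
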(event Custom|Timer
  (if (== (Variables|Default|GetSeconds) 0)
    (if (== (Variables|Default|GetMinutes) 0)
      (Variables|Default|SetbGameOver true)
      (else
        (Variables|Default|SetSeconds 0)
        (Math|Integer|DecrementInt (Variables|Default|GetMinutes))))
    (else
      (Math|Integer|DecrementInt (Variables|Default|GetSeconds)))))

(event EventBeginPlay
  (Utilities|Time|SetTimerbyEvent (delegate Custom|Timer) 1.0 true)
  (Variables|/Script/Engine.PlayerController|SetbShowMouseCursor (Game|GetPlayerController 0) false))

(fn ConstructionScript)