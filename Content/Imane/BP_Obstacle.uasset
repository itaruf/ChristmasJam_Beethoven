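; BP_Obstacle is an obstacle actor that starts a series of quick-time events when the first-person character overlaps it.
; A looping timer polls the player's event state and, whenever the game mode reports a QTE ended, starts another with a random key from the player.
; Clearing the set count destroys the obstacle.
; A failed QTE, or leaving before success, stops the timer, reports failure and removes the widget.
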(event Custom|QTE
  (bind _player (Variables|Default|GetPlayer))
  (bind _currentevent (Variables|/Game/FirstPersonCPP/Blueprints/FirstPersonCharacter.FirstPersonCharacter_C|GetCurrentEvent _player))
  (bind _state (Utilities|Struct|Breaks_EventInfo _currentevent))
  ;[1 1 1] Repeat QTE Every X Seconds
  (Utilities|IsValid _player
    (:Is%20Valid
      (switch Utilities|FlowControl|Switch|Switchone_EventState _state
        (:NewEnumerator0
          (if (Variables|/Game/Imane/BP_GMB.BP_GMB_C|GetbQTEended (Variables|Default|GetGMB)) :!label _label
            (Math|Integer|DecrementInt (Variables|Default|GetNumberOfQTELeft)
              (:%20%20
                (Variables|/Game/Imane/BP_GMB.BP_GMB_C|SetbQTEended (Variables|Default|GetGMB) false)
                (if (== (Variables|Default|GetNumberOfQTELeft) 0)
                  ;[1 1 1] If The Player Has Cleared All QTE - Destroy The Obstacle
                  (Utilities|Time|ClearandInvalidateTimerbyHandle (Variables|Default|GetLoop))
                  (Actor|DestroyActor)
                  (else
                    ;[1 1 1] Start QTE With Key To Press
                    (Default|StartQTE (Variables|Default|GetGMB) (Variables|Default|GetPlayer) (.OutItem (Utilities|Array|Random (Variables|Default|GetRandom%20Keys))) (Variables|Default|GetEventWidgetPosition) (Variables|Default|GetTime) 1.0)))))))
        (:NewEnumerator1
          (goto _label))
        (:NewEnumerator2
          (goto _label))
        (:NewEnumerator3
          (CallFunction|Failure _state))
        (:NewEnumerator4
          (CallFunction|Failure _state))))))

(event Collision|EventActorBeginOverlap
  (params (OtherActor :type Actor%20Object%20Reference))
  ;[1 1 1] Actor Begin Overlap - Start QTE
  (bind _asfirst_person_character (Utilities|Casting|CastToFirstPersonCharacter OtherActor))
  (Variables|Default|SetPlayer _asfirst_person_character)
  (Utilities|FlowControl|Sequence
    (:then_0
      ;[1 1 1] Reset State When Entering
      (Utilities|IsValid (Variables|Default|GetPlayer)
        (:Is%20Valid
          (Utilities|Struct|Setmembersins_EventInfo (Variables|/Game/FirstPersonCPP/Blueprints/FirstPersonCharacter.FirstPersonCharacter_C|GetCurrentEvent (Variables|Default|GetPlayer)) "NewEnumerator0"))))
    (:then_1
      (Variables|Default|SetNumberOfQTELeft (+ (Variables|Default|GetNumberOfQTE) 1))
      (Variables|Default|SetEventWidgetPosition (Utilities|Struct|Makes_EventWidgetPosition (Utilities|Struct|MakeAnchors "(X=0.500000,Y=0.500000)" "(X=0.500000,Y=0.500000)") "(X=0.500000,Y=0.500000)" "(X=0.000000,Y=0.000000)")))
    (:then_2
      ;[1 1 1] Repeat QTE Every X Seconds
      (bind _returnvalue (Utilities|Time|SetTimerbyEvent (delegate Custom|QTE) 0.5 true))
      (Variables|Default|SetLoop _returnvalue))))

(event EventBeginPlay
  ;[1 1 1] Retrieve Data
  (Utilities|FlowControl|Sequence
    (:then_0
      (bind _asfirst_person_character (Utilities|Casting|CastToFirstPersonCharacter (Pawn|GetControlledPawn (Game|GetPlayerController 0))))
      (Variables|Default|SetPlayer _asfirst_person_character)
      (bind _asbp_gmb (Utilities|Casting|CastToBP_GMB (Game|GetGameMode)))
      (Variables|Default|SetGMB _asbp_gmb))
    (:then_1
      (Variables|Default|SetRandom%20Keys (Variables|/Game/FirstPersonCPP/Blueprints/FirstPersonCharacter.FirstPersonCharacter_C|GetRandomKeys (Variables|Default|GetPlayer))))))

(event Collision|EventActorEndOverlap
  (params (OtherActor :type Actor%20Object%20Reference))
  ;[1 1 1] Actor End Overlap - Stop QTE > Set State To Failure
  (Variables|Default|SetNumberOfQTELeft (+ (Variables|Default|GetNumberOfQTE) 1))
  (Utilities|FlowControl|Sequence
    (:then_0
      (bind _asfirst_person_character (Utilities|Casting|CastToFirstPersonCharacter OtherActor))
      (Variables|Default|SetPlayer _asfirst_person_character)
      (bind _asbp_gmb (Utilities|Casting|CastToBP_GMB (Game|GetGameMode)))
      (Variables|Default|SetGMB _asbp_gmb))
    (:then_1
      (switch Utilities|FlowControl|Switch|Switchone_EventState (Utilities|Struct|Breaks_EventInfo (Variables|/Game/FirstPersonCPP/Blueprints/FirstPersonCharacter.FirstPersonCharacter_C|GetCurrentEvent (Variables|Default|GetPlayer)))
        (:NewEnumerator0
          _)
        (:NewEnumerator1
          _)
        (:NewEnumerator3
          _)
        (:NewEnumerator4
          _))
      (Default|OnEventCompleted (Variables|Default|GetPlayer) "NewEnumerator3")
      (CallFunction|Failure "NewEnumerator3"))))

(fn ConstructionScript)

(fn Failure
  (params (State :type e_EventState%20Enum :default "NewEnumerator0"))
  (bind _player (Variables|Default|GetPlayer))
  (bind _eventwidget (Variables|/Game/FirstPersonCPP/Blueprints/FirstPersonCharacter.FirstPersonCharacter_C|GetEventWidget _player))
  (Default|OnEventCompleted (Variables|Default|GetPlayer) State)
  (Utilities|FlowControl|Sequence
    (:then_0
      (Variables|/Game/Imane/BP_GMB.BP_GMB_C|SetbQTEended (Variables|Default|GetGMB) true)
      (if (Utilities|Time|IsValidTimerHandle (Variables|Default|GetLoop))
        (Utilities|Time|ClearandInvalidateTimerbyHandle (Variables|Default|GetLoop))))
    (:then_1
      (Utilities|IsValid _eventwidget
        (:Is%20Valid
          (Widget|RemovefromParent _eventwidget))))))